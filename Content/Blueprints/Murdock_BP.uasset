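; Murdock character Blueprint that adjusts the mesh's aiming pose and prints damage and health events for debugging.
; Every Tick sets the mesh's relative yaw to one of two offsets depending on InADSMode.
; Damage and AttributeComp health delegates only print their values to screen.
; Unconnected leftover branches toggle controller yaw by ADS or velocity and duplicate the mesh rotation, but never run.
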(event TestDeligate(AttributeComp)
  (params (Damage :type Float%20%28single-precision%29))
  (Development|PrintString (Utilities|String|ToString(Float) Damage)))

(event OnHealthChangeAtrriBute(AttributeComp)
  (params (InstigatorActor :type Actor%20Object%20Reference) (OwningComp :type Character%20Attribute%20Component%20Object%20Reference) (NewHealth :type Float%20%28single-precision%29) (Delta :type Float%20%28single-precision%29))
  (Development|PrintString (Utilities|String|ToString(Float) Delta)))

(event EventOnGettingDamageFunction
  (params (AttributeComponent :type Character%20Attribute%20Component%20Object%20Reference) (Healthh :type Float%20%28single-precision%29) (HealthDelta :type Float%20%28single-precision%29) (DamageType :type Damage%20Type%20Object%20Reference) (InstigatedBy :type Controller%20Object%20Reference) (DamageCauser :type Actor%20Object%20Reference))
  (Development|PrintString (Utilities|String|ToString(Float) HealthDelta)))

(event EventTick
  (params (DeltaSeconds :type Float%20%28single-precision%29))
  (Utilities|FlowControl|Sequence
    (:then_0
      (if (Variables|Default|GetbInADSMode)
        (Transformation|SetRelativeRotation (Variables|Character|GetMesh) "0,-70.000000, 0" false false)
        (else
          (Transformation|SetRelativeRotation (Variables|Character|GetMesh) "0,-90.000000, 0" false false))))))

(fn ConstructionScript)