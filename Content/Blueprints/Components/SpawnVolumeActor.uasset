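; Spawn volume actor that scatters weapon pickups at random spots inside its box when play begins.
; On BeginPlay it loops SpawnCount times, picking each location with a helper that wraps RandomPointInBoundingBox around the root position and box extent.
; Each spawned Pickup_Weapon_BP is initialized with a hardcoded weapon ID, so every pickup receives the same one.
; Tick and overlap events are unused.
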(event Collision|EventActorBeginOverlap
  (params (OtherActor :type Actor%20Object%20Reference)))

(event EventTick
  (params (DeltaSeconds :type Float%20%28single-precision%29)))

(event EventBeginPlay
  (for _index (range 1 (Variables|Default|GetSpawnCount))
    (bind _randompoint (CallFunction|NewFunction0 (Transformation|GetWorldLocation (Variables|Default|GetDefaultSceneRoot)) (Variables|/Script/Engine.BoxComponent|GetBoxExtent (Variables|Default|GetBox))))
    (bind _returnvalue (Game|SpawnActorfromClass "/Game/Blueprints/Pickup_Weapon_BP.Pickup_Weapon_BP_C" (Math|Transform|MakeTransform _randompoint "0, 0, 0" "1.000000,1.000000,1.000000") "Undefined" 0 "1" "" 0 0))
    (Class|PickupWeapon|InitPickupWeapon _returnvalue "1")))

(fn ConstructionScript)

(fn NewFunction0
  (params (Center :type Vector) (HalfSize :type Vector))
  (return (Math|Random|RandomPointinBoundingBox Center HalfSize)))