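; SpawnVolumeComp is a component that spawns actors at random points around its owner on BeginPlay.
; It passes the found CoreCharacter_BP to SpawnActor, which repeatedly spawns that actor's class, ignoring collision.
; Points range from the owner's location to location plus scale in X and Y, with Z fixed at their sum.
; It prints each point and initializes only spawns that cast to Pickup_Weapon_BP.
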(event EventBeginPlay
  (bind _returnvalue (Actor|GetActorOfClass "/Game/Blueprints/CoreCharacter_BP.CoreCharacter_BP_C"))
  (CallFunction|SpawnActor _returnvalue 5))

(fn SpawnActor
  (params (ActorToSpawn :type Actor%20Object%20Reference) (SpawnCount :type Integer))
  (bind _returnvalue (Components|GetOwner))
  (bind _returnvalue_2 (Transformation|GetActorScale3D _returnvalue))
  (bind _returnvalue_3 (Transformation|GetActorLocation _returnvalue))
  (for _index (range 0 SpawnCount)
    (bind _output_get (Variables|Default|SetSpawnLocation (Math|Vector|MakeVector (Math|Random|RandomFloatinRange (.x _returnvalue_3) (+ (.x _returnvalue_3) (.x _returnvalue_2))) (Math|Random|RandomFloatinRange (.y _returnvalue_3) (+ (.y _returnvalue_3) (.y _returnvalue_2))) (+ (.z _returnvalue_3) (.z _returnvalue_2)))))
    (Development|PrintString (Utilities|String|ToString(Vector) _output_get) true true "(R=0.000000,G=0.660000,B=1.000000,A=1.000000)" 1e+01)
    (bind _returnvalue_4 (Game|SpawnActorfromClass (Utilities|GetClass ActorToSpawn) (Math|Transform|MakeTransform _output_get "0, 0, 0" "1.000000,1.000000,1.000000") "AlwaysSpawn" 0 0))
    (bind _aspickup_weapon_bp (Utilities|Casting|CastToPickup_Weapon_BP _returnvalue_4))
    (Class|PickupWeapon|InitPickupWeapon _aspickup_weapon_bp "1")))